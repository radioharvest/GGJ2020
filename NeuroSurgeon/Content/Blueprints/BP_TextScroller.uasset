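; BP_TextScroller is an actor that shows a sequence of text strings one at a time on a TextRender component.
; BeginPlay displays the first entry of the Text array and starts a looping five-second timer.
; Each timer tick advances TextIndex and updates the displayed text, then clears the timer once the last entry is shown.
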(event `self.ReceiveBeginPlay`
  (`TextRenderComponent.K2_SetText` (`self.TextRender`) (`KismetTextLibrary.Conv_StringToText` (`|GetArrayItem` (`self.Text`))))
  (bind _returnvalue (`KismetSystemLibrary.K2_SetTimerDelegate` (delegate `TimerOver`) 5.0 true))
  (set `self.Timer` _returnvalue))

(event `TimerOver`
  (bind _returnvalue (+ (`self.TextIndex`) 1))
  (if (< _returnvalue (`KismetArrayLibrary.Array_Length` (`self.Text`)))
    (bind _output_get (set `self.TextIndex` _returnvalue))
    (`TextRenderComponent.K2_SetText` (`self.TextRender`) (`KismetTextLibrary.Conv_StringToText` (`|GetArrayItem` (`self.Text`) _output_get)))
    (else
      (`KismetSystemLibrary.K2_ClearAndInvalidateTimerHandle` (`self.Timer`)))))

(fn `UserConstructionScript`)