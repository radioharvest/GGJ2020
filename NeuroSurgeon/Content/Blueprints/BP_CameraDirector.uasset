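; Camera director that switches which scene capture in a list shows on a shared render target, starting with index 0.
; SwitchToCamera bounds-checks the index, clears the target, assigns it to the chosen SceneCaptureComponent2D and tracks it as current.
; Previous captures keep the target, so capture sort priority is swapped to favor the new one.
; W and S step a test index for debug switching, with printed feedback.
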(event `self.ReceiveBeginPlay`
  (`self.SwitchToCamera` 0))

(event `Key|W`
  (params (Key :type "Key Structure"))
  (bind _testindex (`self.TestIndex`))
  (:`Pressed`
    (set `self.TestIndex` (+ (`self.TestIndex`) 1))
    (`self.SwitchToCamera` _testindex :!label _label)
    (`KismetSystemLibrary.PrintString` (`KismetStringLibrary.Conv_IntToString` _testindex))))

(event `Key|S`
  (params (Key :type "Key Structure"))
  (:`Pressed`
    (set `self.TestIndex` (- (`self.TestIndex`) 1))
    (goto _label)))

(fn `SwitchToCamera`
  (params (Index :type Integer))
  (bind _captures (`self.Captures`))
  (bind _currentcapture (`self.CurrentCapture`))
  (bind _rendertarget (`self.RenderTarget`))
  (bind _output (`|GetArrayItem` _captures Index))
  (bind _returnvalue (`self.GetComponentByClass` _output "/Script/Engine.SceneCaptureComponent2D"))
  (if (and (< Index (`KismetArrayLibrary.Array_Length` _captures)) (>= Index 0))
    (`KismetRenderingLibrary.ClearRenderTarget2D` _rendertarget (struct :`R` 0.041134 :`B` 1.0 :`A` 1.0))
    (set `SceneCaptureComponent2D.TextureTarget` _rendertarget _returnvalue)
    (`/Engine/EditorBlueprintResources/StandardMacros.IsValid` _currentcapture
      (:`Is Valid`
        (`SceneCaptureComponent.SetCaptureSortPriority` _currentcapture 5))
      (:`Is Not Valid`
        _))
    (`SceneCaptureComponent.SetCaptureSortPriority` _returnvalue 0)
    (set `self.CurrentCapture` _returnvalue)
    (`KismetSystemLibrary.PrintString` (`KismetSystemLibrary.GetObjectName` _output))
    (else
      (`KismetSystemLibrary.PrintString` "falzo"))))

(fn `UserConstructionScript`)