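; Needle actor that is aimed around a Brain sphere and pushed into it.
; Axis inputs rotate the root around neutral angles, while ApplyPush slides the mesh along local Z from surface offset to insertion depth.
; Tick places a targeting marker by line-tracing only the brain sphere component toward the root, falling back to the brain radius on a miss.
; Once IsNeedleInside detects penetration, aiming locks and the marker hides.
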(event `self.ReceiveTick`
  (params (DeltaSeconds :type "Float (single-precision)"))
  (bind _targetingposition (`self.TargetingPosition`))
  (bind _targetingposition_2 (`self.TargetingPosition`))
  (if (`self.IsNeedleInside`)
    (`SceneComponent.SetVisibility` _targetingposition false false)
    (else
      (`SceneComponent.SetVisibility` _targetingposition true false)
      (bind (_hitlocation _hitnormal _bonename _outhit _returnvalue) (`PrimitiveComponent.K2_LineTraceComponent` (`/Game/Blueprints/Brain.BrainSphere` (`self.Brain`)) (`SceneComponent.K2_GetComponentLocation` (`self.RaycastStart`)) (`SceneComponent.K2_GetComponentLocation` (`self.DefaultSceneRoot`)) true false false))
      (if _returnvalue
        (`SceneComponent.K2_SetWorldLocation` _targetingposition_2 _hitlocation false true)
        (else
          (`SceneComponent.K2_SetRelativeLocation` _targetingposition_2 (`KismetMathLibrary.MakeVector` 0.0 0.0 (`/Game/Blueprints/Brain.GetBrainRadius` (`self.Brain`))) false true))))))

(fn `Apply Axis Movement Y`
  (params (DeltaY :type "Float (double-precision)"))
  (if (not (`self.IsNeedleInside`))
    (`SceneComponent.K2_SetRelativeRotation` (`self.DefaultSceneRoot`) (`KismetMathLibrary.MakeRotator` (.roll (`SceneComponent.RelativeRotation` (`self.DefaultSceneRoot`))) (+ (`self.NeutralPosY`) DeltaY) (.yaw (`SceneComponent.RelativeRotation` (`self.DefaultSceneRoot`)))) false true)))

(fn `ApplyAxisMovementX`
  (params (DeltaX :type "Float (double-precision)"))
  (if (not (`self.IsNeedleInside`))
    (`SceneComponent.K2_SetRelativeRotation` (`self.DefaultSceneRoot`) (`KismetMathLibrary.MakeRotator` (+ DeltaX (`self.NeutralPosX`)) (.pitch (`SceneComponent.RelativeRotation` (`self.DefaultSceneRoot`))) (.yaw (`SceneComponent.RelativeRotation` (`self.DefaultSceneRoot`)))) false true)))

(fn `ApplyPush`
  (params (PushAmount :type "Float (double-precision)"))
  (bind _returnvalue (- (`self.PositionOffset`) (`self.InsertionDepth`)))
  (`self.SetNeedleOffset` (+ (* (- 1.0 PushAmount) (- (`self.DefaultSurfaceOffset`) _returnvalue)) _returnvalue (`/Game/Blueprints/Brain.GetBrainRadius` (`self.Brain`)))))

(fn `IsNeedleInside`
  (returns (IsNeedleInside :type Boolean))
  (return (< (.z (`SceneComponent.RelativeLocation` (`self.NeedleMesh`))) (+ (`self.PositionOffset`) (`/Game/Blueprints/Brain.GetBrainRadius` (`self.Brain`))))))

(fn `SetNeedleOffset`
  (params (Offset :type "Float (double-precision)"))
  (`SceneComponent.K2_SetRelativeLocation` (`self.NeedleMesh`) (`KismetMathLibrary.MakeVector` 0.0 0.0 Offset) false true))

(fn `UserConstructionScript`
  (set `self.PositionOffset` (`KismetMathLibrary.VSize` (- (`SceneComponent.K2_GetComponentLocation` (`self.NeedleMesh`)) (`SceneComponent.K2_GetComponentLocation` (`self.RaycastStart`)))))
  (`SceneComponent.K2_SetRelativeRotation` (`self.DefaultSceneRoot`) (`KismetMathLibrary.MakeRotator` (`self.NeutralPosX`) (`self.NeutralPosY`)) false false)
  (`self.SetNeedleOffset` (+ (`self.DefaultSurfaceOffset`) (`/Game/Blueprints/Brain.GetBrainRadius` (`self.Brain`))))
  (`SceneComponent.K2_SetRelativeLocation` (`self.TargetingPosition`) (`KismetMathLibrary.MakeVector` 0.0) false true))