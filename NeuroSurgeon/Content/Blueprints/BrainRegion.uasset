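; BrainRegion highlights a brain region's mesh when a needle overlaps it, glowing by penetration depth.
; Each Tick with a valid OverlappingNeedle tints the first child static mesh with Color, sets Emissive to the depth and prints it.
; It then clears the needle reference, so the mesh turns black and unlit next Tick unless the reference is set again externally.
; Both branches create and assign a dynamic material instance every frame.
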(event `self.ReceiveTick`
  (params (DeltaSeconds :type "Float (single-precision)"))
  (bind _depth (`/Game/Blueprints/Needle.PenetrationDepth` (`self.OverlappingNeedle`)))
  (if (`KismetSystemLibrary.IsValid` (`self.OverlappingNeedle`))
    (bind _asstatic_mesh_component (cast `StaticMeshComponent` (`self.GetChildComponent` self 0)))
    (bind _returnvalue (`PrimitiveComponent.CreateDynamicMaterialInstance` _asstatic_mesh_component 0 (`|GetArrayItem` (`MeshComponent.GetMaterials` _asstatic_mesh_component)) "None"))
    (`MaterialInstanceDynamic.SetVectorParameterValue` _returnvalue "RandomColor" (`KismetMathLibrary.Conv_ColorToLinearColor` (`self.Color`)))
    (`MaterialInstanceDynamic.SetScalarParameterValue` _returnvalue "Emissive" _depth)
    (`KismetSystemLibrary.PrintString` (`KismetStringLibrary.Conv_DoubleToString` _depth))
    (`PrimitiveComponent.SetMaterial` _asstatic_mesh_component 0 _returnvalue)
    (set `self.OverlappingNeedle` null)
    (else
      (bind _asstatic_mesh_component_2 (cast `StaticMeshComponent` (`self.GetChildComponent` self 0)))
      (bind _returnvalue_2 (`PrimitiveComponent.CreateDynamicMaterialInstance` _asstatic_mesh_component_2 0 null "None"))
      (`MaterialInstanceDynamic.SetVectorParameterValue` :`self` _returnvalue_2 :`ParameterName` "RandomColor")
      (`MaterialInstanceDynamic.SetScalarParameterValue` _returnvalue_2 "Emissive" 0.0)
      (`PrimitiveComponent.SetMaterial` _asstatic_mesh_component_2 0 _returnvalue_2))))